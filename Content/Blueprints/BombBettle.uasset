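; BombBettle is a kamikaze-style enemy that chases the first-person player and damages them on contact.
; When its PawnSensing component sees a FirstPersonCharacter, it uses AI Move To to head for that character.
; On overlapping the player, it applies a fixed amount of damage and destroys itself.
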(event OnSeePawn(PawnSensing)
  (params (Pawn :type Pawn%20Object%20Reference))
  (bind _asfirst_person_character (Utilities|Casting|CastToFirstPersonCharacter Pawn))
  (AI|AIMoveTo self "0, 0, 0" _asfirst_person_character 5.0 false))

(event EventBeginPlay)

(event Collision|EventActorBeginOverlap
  (params (OtherActor :type Actor%20Object%20Reference))
  ;[1 1 1] Enemy overlapping player
  (Utilities|Casting|CastToFirstPersonCharacter OtherActor)
  (Game|Damage|ApplyDamage OtherActor 3e+01 0 0 "/Script/Engine.DamageType")
  (Actor|DestroyActor))

(event EventTick
  (params (DeltaSeconds :type Float%20%28single-precision%29))
  (|CallParentFunction DeltaSeconds) ; This node is disabled and will not be called.\nDrag off pins to build functionality.
)

(fn ConstructionScript
  (|CallParentFunction))