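; TestEnemy is a test enemy that chases the player and dies when shot.
; PawnSensing triggers an AI move toward any FirstPersonCharacter it sees.
; DefaultBullet hits on the Cube component print debug text, subtract bullet damage from Health only on the authority, and play a hitmarker sound.
; At zero Health or below, it spawns an explosion emitter and destroys itself.
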(event OnSeePawn(PawnSensing)
  (params (Pawn :type Pawn%20Object%20Reference))
  (bind _asfirst_person_character (Utilities|Casting|CastToFirstPersonCharacter Pawn))
  (AI|AIMoveTo self "0, 0, 0" _asfirst_person_character 5.0 false))

(event OnComponentHit(Cube)
  (params (HitComponent :type Primitive%20Component%20Object%20Reference) (OtherActor :type Actor%20Object%20Reference) (OtherComp :type Primitive%20Component%20Object%20Reference) (NormalImpulse :type Vector :default "0, 0, 0") (Hit :type Hit%20Result%20Structure%20%28by%20ref%29))
  (bind _asdefault_bullet (Utilities|Casting|CastToDefaultBullet OtherActor))
  (Development|PrintText "HIIT")
  (Networking|SwitchHasAuthority
    (:Authority
      (bind _output_get (Variables|Default|SetHealth (- (Variables|Default|GetHealth) (Variables|/Game/Blueprints/DefaultBullet.DefaultBullet_C|GetDamage _asdefault_bullet)))))
    (:Remote
      _))
  (Audio|PlaySound2D "/Game/Audio/Hitmarker.Hitmarker" 1.0 1.0 0.0 0 0)
  (if (<= _output_get 0.0)
    (Effects|SpawnEmitteratLocation "/Game/StarterContent/Particles/P_Explosion.P_Explosion" (Transformation|GetActorLocation))
    (Actor|DestroyActor)))

(fn ConstructionScript)