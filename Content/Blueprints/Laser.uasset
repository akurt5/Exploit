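; Laser is a projectile actor that damages what it hits and destroys itself on impact.
; On a collision hit, actors tagged Hittable take the Damage value and trigger a 2D hitmarker sound.
; Hittable actors also tagged Relic spawn an extra relic shatter effect.
; Every hit, tagged or not, spawns a bullet shatter emitter at the laser's location before the actor is destroyed.
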(event OnComponentHit(CollisionComponent)
  (params (HitComponent :type Primitive%20Component%20Object%20Reference) (OtherActor :type Actor%20Object%20Reference) (OtherComp :type Primitive%20Component%20Object%20Reference) (NormalImpulse :type Vector :default "0, 0, 0") (Hit :type Hit%20Result%20Structure%20%28by%20ref%29))
  (bind _hitactor (Collision|BreakHitResult Hit))
  (if (Actor|ActorHasTag _hitactor "Hittable")
    (if (Actor|ActorHasTag _hitactor "Relic")
      (Effects|SpawnEmitteratLocation "/Game/Particles/RelicShatter.RelicShatter" (Transformation|GetActorLocation)))
    (Audio|PlaySound2D "/Game/Audio/Hitmarker.Hitmarker" 0.3 1.0 0.0 0 0)
    (Game|Damage|ApplyDamage _hitactor (Variables|Default|GetDamage) 0 0))
  (Effects|SpawnEmitteratLocation "/Game/Particles/BulletShatter.BulletShatter" (Transformation|GetActorLocation))
  (Actor|DestroyActor))

(fn ConstructionScript)