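; ShootingEnemy is an enemy actor that fires one homing laser at the player when play begins.
; BeginPlay calls SpawnProjectile, which spawns a Laser at the enemy's location, rotated toward player character 0 and stretched along Z.
; The spawned laser's projectile component is then set to home in on the player character's mesh.
; Tick and overlap events are disabled, so it never fires again on its own.
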(event EventBeginPlay
  (CallFunction|SpawnProjectile))

(event Collision|EventActorBeginOverlap
  (params (OtherActor :type Actor%20Object%20Reference)))

(event EventTick
  (params (DeltaSeconds :type Float%20%28single-precision%29)))

(fn ConstructionScript
  (|CallParentFunction))

(fn SpawnProjectile
  (bind _returnvalue (Game|GetPlayerCharacter 0))
  (bind _returnvalue_2 (Transformation|GetActorLocation))
  (bind _returnvalue_3 (Game|SpawnActorfromClass "/Game/Blueprints/Laser.Laser_C" (Math|Transform|MakeTransform _returnvalue_2 (Math|Rotator|FindLookatRotation _returnvalue_2 (Transformation|GetActorLocation _returnvalue)) "1,1,2.000000") "AdjustIfPossibleButDontSpawnIfColliding" 0 0))
  (Variables|/Script/Engine.ProjectileMovementComponent|SetHomingTargetComponent (Variables|/Game/Blueprints/Laser.Laser_C|GetProjectile _returnvalue_3) (Variables|/Script/Engine.Character|GetMesh _returnvalue))
  (Variables|/Script/Engine.ProjectileMovementComponent|SetbIsHomingProjectile (Variables|/Game/Blueprints/Laser.Laser_C|GetProjectile _returnvalue_3) true))