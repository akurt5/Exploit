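; BaseEnemy is an enemy Blueprint that takes damage, grants experience when killed and explodes on destruction.
; AnyDamage subtracts damage from Health and, at zero or below, loops over all FirstPersonCharacter actors, adding EnemyExpToGive to each one's Exp.
; DestroyActor is called inside that loop, so destruction depends on at least one character being found.
; The Destroyed event spawns the P_Explosion emitter at the actor's location.
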(event Game|Damage|EventAnyDamage
  (params (Damage :type Float%20%28single-precision%29) (DamageType :type Damage%20Type%20Object%20Reference) (InstigatedBy :type Controller%20Object%20Reference) (DamageCauser :type Actor%20Object%20Reference))
  (bind _output_get (Variables|Default|SetHealth (- (Variables|Default|GetHealth) Damage)))
  (if (<= _output_get 0.0)
    (bind _outactors (Actor|GetAllActorsOfClass "/Game/Blueprints/FirstPersonCharacter.FirstPersonCharacter_C"))
    (for _array_element _outactors
      (Variables|/Game/Blueprints/FirstPersonCharacter.FirstPersonCharacter_C|SetExp _array_element (+ (Variables|/Game/Blueprints/FirstPersonCharacter.FirstPersonCharacter_C|GetExp _array_element) (Variables|Default|GetEnemyExpToGive)))
      (Actor|DestroyActor))))

(event EventDestroyed
  (Effects|SpawnEmitteratLocation "/Game/StarterContent/Particles/P_Explosion.P_Explosion" (Transformation|GetActorLocation)))

(fn ConstructionScript)