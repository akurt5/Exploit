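; SpawnPoint is an enemy spawner that endlessly spawns ShootingEnemy actors at its own transform.
; On BeginPlay, only the authority waits a random initial delay, then enters a spawn-and-delay loop.
; Each pass decrements the Min and Max variables and draws the next random delay from their clamped values, so spawns grow more frequent over time down to a fixed floor.
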(event EventBeginPlay
  (Networking|SwitchHasAuthority
    (:Authority
      (Utilities|FlowControl|Delay (Math|Random|RandomFloatinRange 1.0 2e+01))
      (Game|SpawnActorfromClass "/Game/Blueprints/ShootingEnemy.ShootingEnemy_C" (Transformation|GetActorTransform) "Undefined" 0 0 :!label _label)
      (bind _result (Math|Float|DecrementFloat (Variables|Default|Getmin))
        (:%20%20
          (bind _result_2 (Math|Float|DecrementFloat (Variables|Default|Getmax))
            (:%20%20
              (Utilities|FlowControl|Delay (Math|Random|RandomFloatinRange (Math|Float|Clamp(Float) _result 3.0 2e+01) (Math|Float|Clamp(Float) _result_2 5.0 3e+01)))
              (goto _label))))))))

(fn ConstructionScript)